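; MyGameInstance holds score, bill and next-level state, apparently as the game instance that carries it between levels.
; It reads the current score from the first GameManager actor in the level and stores a next level to load.
; At level end it computes the round total as total score plus that score minus the bill.
; Helpers raise the bill by a fixed step and reset scores and bill to starting values.
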(fn SetScoretoAdd
  (bind _outactors (Actor|GetAllActorsOfClass "/Game/MyContent/Blueprints/GameManager.GameManager_C"))
  (Variables|Default|SetScoreToAdd (Variables|/Game/MyContent/Blueprints/GameManager.GameManager_C|GetScore (Utilities|Array|Get(acopy) _outactors))))

(fn SetNextLevel
  (params (NextLevel :type Name))
  (Variables|Default|SetNextLevelToLoad NextLevel))

(fn EndLevelAdding
  (Variables|Default|SetAllRoundTotal (- (+ (Variables|Default|GetTotalScore) (Variables|Default|GetScoreToAdd)) (Variables|Default|GetBill))))

(fn IncreaseBill
  (Variables|Default|SetBill (+ (Variables|Default|GetBill) 10)))

(fn Clear
  (Variables|Default|SetTotalScore 0)
  (Variables|Default|SetScoreToAdd 0)
  (Variables|Default|SetAllRoundTotal 0)
  (Variables|Default|SetBill 50))