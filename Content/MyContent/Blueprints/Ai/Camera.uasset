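; Security camera AI actor that triggers game over through the GameManager when its line of sight detects a pawn while IsHiden is false.
; Every Tick it traces for Pawn objects to a sweeping end point, ignoring all AI actors.
; A Running-gated Delay loop swings that point down-left, center, down-right and back along X, swapping the guard sprite at each TimeSwitch interval.
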(event EventTick
  (params (DeltaSeconds :type Float%20%28single-precision%29))
  (bind _self self)
  (bind _timeswitch (Variables|Default|GetTimeSwitch))
  (bind _papersprite (Variables|Default|GetPaperSprite))
  (bind _returnvalue (Transformation|GetActorLocation _self))
  (bind _outactors (Actor|GetAllActorsOfClass "/Game/MyContent/Blueprints/Ai/AI.AI_C"))
  (bind _returnvalue_2 (Collision|LineTraceForObjects _returnvalue (Variables|Default|Getend) (Utilities|Array|MakeArray "ObjectTypeQuery3") false _outactors "None" true "(R=1.000000,G=0.000000,B=0.000000,A=1.000000)" "(R=0.000000,G=1.000000,B=0.000000,A=1.000000)" 0.0))
  (Utilities|FlowControl|Sequence
    (:then_0
      (if (not (Variables|Default|GetisHiden))
        (if _returnvalue_2
          (bind _outactors_2 (Actor|GetAllActorsOfClass "/Game/MyContent/Blueprints/GameManager.GameManager_C"))
          (Default|Setgameover (Utilities|Array|Get(acopy) _outactors_2)))))
    (:then_1
      (if (not (Variables|Default|Getrunning))
        (Variables|Default|Setrunning true)
        (Variables|Default|Setend (+ _returnvalue "-40.000000, 0,-40.000000"))
        (Rendering|Components|Sprite|SetSprite _papersprite "/Game/MyContent/Sprits/CharGaurd_Sprite_12.CharGaurd_Sprite_12")
        (Utilities|FlowControl|Delay _timeswitch)
        (Variables|Default|Setend (+ _returnvalue "0.000000, 0,-40.000000"))
        (Rendering|Components|Sprite|SetSprite _papersprite "/Game/MyContent/Sprits/CharGaurd_Sprite_14.CharGaurd_Sprite_14")
        (Utilities|FlowControl|Delay _timeswitch)
        (Variables|Default|Setend (+ _returnvalue "40.000000, 0,-40.000000"))
        (Rendering|Components|Sprite|SetSprite _papersprite "/Game/MyContent/Sprits/CharGaurd_Sprite_13.CharGaurd_Sprite_13")
        (Utilities|FlowControl|Delay _timeswitch)
        (Variables|Default|Setend (+ _returnvalue "0.000000, 0,-40.000000"))
        (Rendering|Components|Sprite|SetSprite _papersprite "/Game/MyContent/Sprits/CharGaurd_Sprite_14.CharGaurd_Sprite_14")
        (Utilities|FlowControl|Delay _timeswitch)
        (Variables|Default|Setrunning false)))))

(fn ConstructionScript)