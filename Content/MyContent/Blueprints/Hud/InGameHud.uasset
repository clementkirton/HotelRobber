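; InGameHud puts the screen widget for the current level or game state on the player's viewport.
; BeginPlay picks the end-of-level, main menu, game over or gameplay HUD widget from the level name and GameManager's GameOver flag.
; Outside the end and menu levels, Tick polls GameManager and re-enters that creation step every frame GameOver is true, without removing earlier widgets.
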(event EventBeginPlay
  (bind _returnvalue (Game|GetCurrentLevelName true))
  (bind _returnvalue_2 (UserInterface|CreateWidget (select (Utilities|Enum|Equal(Enum) _returnvalue "LevelEnd") "/Game/MyContent/Blueprints/Hud/EndOfLevel.EndOfLevel_C" (select (Utilities|Enum|Equal(Enum) _returnvalue "MainMenu") "/Game/MyContent/Blueprints/Hud/MainMenuWidget.MainMenuWidget_C" (select (Variables|/Game/MyContent/Blueprints/GameManager.GameManager_C|GetGameOver (Utilities|Array|Get(acopy) (stale EventTick _outactors))) "/Game/MyContent/Blueprints/Hud/GameOver.GameOver_C" "/Game/MyContent/Blueprints/Hud/GameHud.GameHud_C"))) (Game|GetPlayerController 0)))
  (UserInterface|Viewport|AddtoViewport _returnvalue_2 0))

(event EventTick
  (params (DeltaSeconds :type Float%20%28single-precision%29))
  (if (not (or (Utilities|Enum|Equal(Enum) (stale EventBeginPlay _returnvalue) "LevelEnd") (Utilities|Enum|Equal(Enum) (stale EventBeginPlay _returnvalue) "MainMenu")))
    (bind _outactors (Actor|GetAllActorsOfClass "/Game/MyContent/Blueprints/GameManager.GameManager_C"))
    (if (Variables|/Game/MyContent/Blueprints/GameManager.GameManager_C|GetGameOver (Utilities|Array|Get(acopy) _outactors))
      (bind _returnvalue (UserInterface|CreateWidget (select (Utilities|Enum|Equal(Enum) (stale EventBeginPlay _returnvalue) "LevelEnd") "/Game/MyContent/Blueprints/Hud/EndOfLevel.EndOfLevel_C" (select (Utilities|Enum|Equal(Enum) (stale EventBeginPlay _returnvalue) "MainMenu") "/Game/MyContent/Blueprints/Hud/MainMenuWidget.MainMenuWidget_C" (select (Variables|/Game/MyContent/Blueprints/GameManager.GameManager_C|GetGameOver (Utilities|Array|Get(acopy) _outactors)) "/Game/MyContent/Blueprints/Hud/GameOver.GameOver_C" "/Game/MyContent/Blueprints/Hud/GameHud.GameHud_C"))) (Game|GetPlayerController 0)))
      (UserInterface|Viewport|AddtoViewport _returnvalue 0))))

(fn ConstructionScript)