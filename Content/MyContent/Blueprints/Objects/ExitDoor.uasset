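; ExitDoor is a level exit with a flipbook door that the player opens by pressing Interact while overlapping it.
; Overlap events gate the input, and BeginPlay holds the non-looping animation at its first frame until use.
; On use it plays the animation and, after a short delay, passes NextLevel to MyGameInstance, updates the score there and opens LevelEnd.
; Despite a comment mentioning a key, no key check exists.
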(event Collision|EventActorEndOverlap
  (params (OtherActor :type Actor%20Object%20Reference))
  ;[1 1 1] IsPlayerInFrountOfDoor
  (if (== OtherActor (Game|GetPlayerCharacter 0))
    (Variables|Default|SetBI_isOverLap false)))

(event Collision|EventActorBeginOverlap
  (params (OtherActor :type Actor%20Object%20Reference))
  ;[1 1 1] IsPlayerInFrountOfDoor
  (if (== OtherActor (Game|GetPlayerCharacter 0))
    (Variables|Default|SetBI_isOverLap true)))

(event EventBeginPlay
  (bind _door (Variables|Default|GetDoor))
  ;[1 1 1] StopsTheDoorAnimationAtStart
  (Class|PaperFlipbookComponent|SetPlaybackPositioninFrames _door 0 false)
  (Audio|Components|Audio|Stop _door)
  (Components|Timeline|SetLooping _door false))

(event Input|ActionEvents|InputActionInteract
  (params (Key :type Key%20Structure))
  ;[1 1 1] LooksForKeyAndMovesPlayer
  (:Pressed
    (if (Variables|Default|GetBI_isOverLap)
      (Components|Timeline|PlayfromStart (Variables|Default|GetDoor))
      (Utilities|FlowControl|Delay 0.7)
      (bind _asmy_game_instance (Utilities|Casting|CastToMyGameInstance (Game|GetGameInstance))
        (:then
          (Default|SetNextLevel _asmy_game_instance (Variables|Default|GetNextLevel))
          (Default|SetScoretoAdd _asmy_game_instance)
          (Default|EndLevelAdding _asmy_game_instance)
          (Game|OpenLevel(byName) "LevelEnd"))
        (:CastFailed
          (Development|PrintString "Faieled to send the score"))))))

(fn ConstructionScript)