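; SafeDrop is a drop object that adds score to the GameManager when another actor begins overlapping it.
; A short delay after BeginPlay sets a flag that blocks overlaps until spawning settles.
; If the GameManager's item total is within its limit, the overlap adds score, increments that total, plays a 2D sound and destroys the actor.
; The GameManager is found through GetAllActorsOfClass, using the first result.
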(event EventBeginPlay
  (Variables|Default|SetSpawnTimeDone false)
  (Utilities|FlowControl|Delay 0.1)
  (Variables|Default|SetSpawnTimeDone true))

(event Collision|EventActorBeginOverlap
  (params (OtherActor :type Actor%20Object%20Reference))
  (if (Variables|Default|GetSpawnTimeDone)
    (if (<= (Variables|/Game/MyContent/Blueprints/GameManager.GameManager_C|GetTotalItems (Utilities|Array|Get(acopy) (stale _outactors))) 10)
      (bind _outactors (Actor|GetAllActorsOfClass "/Game/MyContent/Blueprints/GameManager.GameManager_C"))
      (Default|AddScore (Utilities|Array|Get(acopy) _outactors) (Variables|Default|GetToAdd))
      (Default|AddTotalItems (Utilities|Array|Get(acopy) _outactors))
      (Audio|PlaySound2D 0)
      (Actor|DestroyActor))))

(fn ConstructionScript)