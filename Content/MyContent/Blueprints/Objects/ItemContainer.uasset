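; Interactable safe container actor that plays its opening animation and drops a SafeDrop actor when the player interacts while overlapping it.
; Overlap sets the PlayerOverlap flag and adds a widget component, removed on exit.
; Interact plays the Safe flipbook, waits briefly, spawns the drop at a random X offset, then sets Spawned to block repeats.
; Releasing Interact also clears PlayerOverlap, so another press requires re-entering the overlap.
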(event Collision|EventActorBeginOverlap
  (params (OtherActor :type Actor%20Object%20Reference))
  (Variables|Default|SetPlayerOverlap true)
  (bind _returnvalue (AddComponent|AddWidgetComponent false)))

(event EventBeginPlay
  (bind _safe (Variables|Default|GetSafe))
  (Class|PaperFlipbookComponent|SetPlaybackPositioninFrames _safe 0 false)
  (Audio|Components|Audio|Stop _safe)
  (Components|Timeline|SetLooping _safe false))

(event Collision|EventActorEndOverlap
  (params (OtherActor :type Actor%20Object%20Reference))
  (Variables|Default|SetPlayerOverlap false)
  (Components|DestroyComponent (stale Collision|EventActorBeginOverlap _returnvalue)))

(event Input|ActionEvents|InputActionInteract
  (params (Key :type Key%20Structure))
  (bind _returnvalue (Transformation|GetActorTransform))
  (bind (_location _rotation _scale) (Math|Transform|BreakTransform _returnvalue))
  (:Pressed
    (if (and (Variables|Default|GetPlayerOverlap) (not (Variables|Default|GetSpawned)))
      (Components|Timeline|PlayfromStart (Variables|Default|GetSafe))
      (Utilities|FlowControl|Delay 0.7)
      (Game|SpawnActorfromClass "/Game/MyContent/Blueprints/Objects/SafeDrop.SafeDrop_C" (Math|Transform|MakeTransform (+ (Math|Vector|MakeVector (Math|Random|RandomFloatinRange -1e+01 5.0) 0.0 -5.0) _location) _rotation _scale) "AdjustIfPossibleButAlwaysSpawn" 0 0)
      (Variables|Default|SetSpawned true)))
  (:Released
    (Variables|Default|SetPlayerOverlap false)))

(fn ConstructionScript)