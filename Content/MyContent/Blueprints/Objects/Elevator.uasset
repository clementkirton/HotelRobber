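; Elevator actor that carries the player to a linked OtherDoor when they press Interact while overlapping it.
; Overlap events set a flag for the player character, gating the input.
; Interact plays the Door animation forward, nudges the actor along Y, reverses the animation, then teleports the pawn beside OtherDoor and resets.
; Fixed delays sequence the steps, and BeginPlay holds the animation at its first frame.
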(event Collision|EventActorEndOverlap
  (params (OtherActor :type Actor%20Object%20Reference))
  (if (== OtherActor (Game|GetPlayerCharacter 0))
    ;[1 1 1] IsPlayerInFrountOfDoor
    (Variables|Default|SetBI_isOverLap false)))

(event Collision|EventActorBeginOverlap
  (params (OtherActor :type Actor%20Object%20Reference))
  (if (== OtherActor (Game|GetPlayerCharacter 0))
    ;[1 1 1] IsPlayerInFrountOfDoor
    (Variables|Default|SetBI_isOverLap true)))

(event EventBeginPlay
  (bind _door (Variables|Default|GetDoor))
  ;[1 1 1] StopsTheDoorAnimationAtStart
  (Class|PaperFlipbookComponent|SetPlaybackPositioninFrames _door 0 false)
  (Audio|Components|Audio|Stop _door)
  (Components|Timeline|SetLooping _door false))

(event Input|ActionEvents|InputActionInteract
  (params (Key :type Key%20Structure))
  (bind _returnvalue (Transformation|GetActorTransform))
  (bind _returnvalue_2 (Transformation|GetActorTransform))
  (bind (_location _rotation _scale) (Math|Transform|BreakTransform _returnvalue))
  (bind (_location_2 _rotation_2 _scale_2) (Math|Transform|BreakTransform _returnvalue_2))
  (:Pressed
    ;[1 1 1] LooksForKeyAndMovesPlayer
    (if (Variables|Default|GetBI_isOverLap)
      (Variables|Default|SetBI_isOverLap false)
      (Components|Timeline|PlayfromStart (Variables|Default|GetDoor))
      (Utilities|FlowControl|Delay 0.7)
      (Transformation|SetActorTransform (Math|Transform|MakeTransform (+ _location_2 "0.000000,4.000000,0.000000") _rotation_2 _scale_2))
      (Utilities|String|Reverse (Variables|Default|GetDoor))
      (Utilities|FlowControl|Delay 0.7)
      (Transformation|Teleport (Pawn|GetControlledPawn (Game|GetPlayerController 0)) (+ (Transformation|GetActorLocation (Variables|Default|GetOtherDoor)) "0.000000,1.000000, 0") "0, 0, 0")
      (Class|PaperFlipbookComponent|SetPlaybackPositioninFrames (Variables|Default|GetDoor) 0 false)
      (Transformation|SetActorTransform (Math|Transform|MakeTransform (+ _location "0.000000,-4.000000,0.000000") _rotation _scale))
      (Variables|Default|SetBI_isOverLap false))))

(fn ConstructionScript)