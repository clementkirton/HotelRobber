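; Hiding-spot object that lets the player hide from AI and cameras.
; Player overlap adds a widget component, and pressing Interact while overlapping starts hiding by setting a hidden flag on every AI and Camera actor.
; Leaving the overlap removes the widget and, if hiding, clears those flags.
; Both state changes nudge the object itself along world Y, in opposite directions.
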(event Collision|EventActorEndOverlap
  (params (OtherActor :type Actor%20Object%20Reference))
  (bind _returnvalue (Transformation|GetActorTransform))
  (bind (_location _rotation _scale) (Math|Transform|BreakTransform _returnvalue))
  (if (== OtherActor (Game|GetPlayerCharacter 0))
    (Variables|Default|SetOverLap false)
    (Components|DestroyComponent (stale Collision|EventActorBeginOverlap _returnvalue))
    (if (not (not (Variables|Default|GetisHideing)))
      (Variables|Default|SetisHideing false)
      (bind _outactors (Actor|GetAllActorsOfClass "/Game/MyContent/Blueprints/Ai/AI.AI_C"))
      (for _array_element _outactors
        (Variables|/Game/MyContent/Blueprints/Ai/AI.AI_C|SetIsHiden _array_element false))
      (bind _outactors_2 (Actor|GetAllActorsOfClass "/Game/MyContent/Blueprints/Ai/Camera.Camera_C"))
      (for _array_element_2 _outactors_2
        (Variables|/Game/MyContent/Blueprints/Ai/Camera.Camera_C|SetisHiden _array_element_2 false))
      (Transformation|SetActorTransform (Math|Transform|MakeTransform (+ _location (Math|Vector|MakeVector 0.0 (select (Variables|Default|GetisHideing) 6.0 -6.0) 0.0)) _rotation _scale)))))

(event Collision|EventActorBeginOverlap
  (params (OtherActor :type Actor%20Object%20Reference))
  (if (== OtherActor (Game|GetPlayerCharacter 0))
    (Variables|Default|SetOverLap true)
    (bind _returnvalue (AddComponent|AddWidgetComponent false))))

(event Input|ActionEvents|InputActionInteract
  (params (Key :type Key%20Structure))
  (bind _returnvalue (Transformation|GetActorTransform))
  (bind (_location _rotation _scale) (Math|Transform|BreakTransform _returnvalue))
  (:Pressed
    (if (and (Variables|Default|GetOverLap) (not (Variables|Default|GetisHideing)))
      (Variables|Default|SetisHideing true)
      (bind _outactors (Actor|GetAllActorsOfClass "/Game/MyContent/Blueprints/Ai/AI.AI_C"))
      (for _array_element _outactors
        (Variables|/Game/MyContent/Blueprints/Ai/AI.AI_C|SetIsHiden _array_element true))
      (bind _outactors_2 (Actor|GetAllActorsOfClass "/Game/MyContent/Blueprints/Ai/Camera.Camera_C"))
      (for _array_element_2 _outactors_2
        (Variables|/Game/MyContent/Blueprints/Ai/Camera.Camera_C|SetisHiden _array_element_2 true))
      (Transformation|SetActorTransform (Math|Transform|MakeTransform (+ _location (Math|Vector|MakeVector 0.0 (select (Variables|Default|GetisHideing) 6.0 -6.0) 0.0)) _rotation _scale)))))

(fn ConstructionScript)