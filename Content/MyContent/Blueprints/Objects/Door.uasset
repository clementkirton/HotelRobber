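; Paired door that teleports the player to a linked OtherDoor and previews the destination while they stand at it.
; Player overlap moves a Camera to an offset from OtherDoor and toggles ShowDoorCam on the GameManager found by class lookup.
; Pressing Interact while overlapping plays the frame-based Door animation, waits briefly, teleports the player's pawn beside OtherDoor, then rewinds the animation.
; BeginPlay holds the animation stopped on its first frame, without looping.
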(event Collision|EventActorEndOverlap
  (params (OtherActor :type Actor%20Object%20Reference))
  ;[1 1 1] IsPlayerInFrountOfDoor
  (if (== OtherActor (Game|GetPlayerCharacter 0))
    (Variables|Default|SetBI_isOverLap false)
    (bind _outactors (Actor|GetAllActorsOfClass "/Game/MyContent/Blueprints/GameManager.GameManager_C"))
    (Variables|/Game/MyContent/Blueprints/GameManager.GameManager_C|SetShowDoorCam (Utilities|Array|Get(acopy) _outactors) false)))

(event Collision|EventActorBeginOverlap
  (params (OtherActor :type Actor%20Object%20Reference))
  (bind _otherdoor (Variables|Default|GetOtherDoor))
  (bind _returnvalue (Transformation|GetActorLocation _otherdoor))
  (bind (_x _y _z) (Math|Vector|BreakVector _returnvalue))
  ;[1 1 1] IsPlayerInFrountOfDoor
  (if (== OtherActor (Game|GetPlayerCharacter 0))
    (Variables|Default|SetBI_isOverLap true)
    (Transformation|SetActorLocation (Variables|Default|GetCamera) (Math|Vector|MakeVector _x (+ _y 65.0) _z) false false)
    (bind _outactors (Actor|GetAllActorsOfClass "/Game/MyContent/Blueprints/GameManager.GameManager_C"))
    (Variables|/Game/MyContent/Blueprints/GameManager.GameManager_C|SetShowDoorCam (Utilities|Array|Get(acopy) _outactors) true)))

(event EventBeginPlay
  (bind _door (Variables|Default|GetDoor))
  ;[1 1 1] StopsTheDoorAnimationAtStart
  (Class|PaperFlipbookComponent|SetPlaybackPositioninFrames _door 0 false)
  (Audio|Components|Audio|Stop _door)
  (Components|Timeline|SetLooping _door false))

(event Input|ActionEvents|InputActionInteract
  (params (Key :type Key%20Structure))
  ;[1 1 1] LooksForKeyAndMovesPlayer
  (:Pressed
    (if (Variables|Default|GetBI_isOverLap)
      (Components|Timeline|PlayfromStart (Variables|Default|GetDoor))
      (Utilities|FlowControl|Delay 0.7)
      (Transformation|Teleport (Pawn|GetControlledPawn (Game|GetPlayerController 0)) (+ (Transformation|GetActorLocation (Variables|Default|GetOtherDoor)) "0,4.000000, 0") "0, 0, 0")
      (Class|PaperFlipbookComponent|SetPlaybackPositioninFrames (Variables|Default|GetDoor) 0 false))))

(fn ConstructionScript)