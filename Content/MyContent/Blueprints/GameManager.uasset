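; GameManager tracks per-round score, collected item count and game-over state.
; On BeginPlay it copies the all-round total into MyGameInstance's TotalScore and calls IncreaseBill on that instance.
; AddScore accumulates Score, and AddTotalItems flags the player's BP_MyChar as having a full bag once the item count reaches its limit.
; Setgameover sets the GameOver flag and pauses the game.
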(event EventBeginPlay
  (bind _asmy_game_instance (Utilities|Casting|CastToMyGameInstance (Game|GetGameInstance)))
  (Variables|/Game/MyContent/Blueprints/MyGameInstance.MyGameInstance_C|SetTotalScore _asmy_game_instance (Variables|/Game/MyContent/Blueprints/MyGameInstance.MyGameInstance_C|GetAllRoundTotal _asmy_game_instance))
  (Default|IncreaseBill _asmy_game_instance))

(fn ConstructionScript)

(fn AddScore
  (params (ToAdd :type Integer))
  (Variables|Default|SetScore (+ (Variables|Default|GetScore) ToAdd)))

(fn Setgameover
  (Variables|Default|SetGameOver true)
  (Game|SetGamePaused true))

(fn AddTotalItems
  (Variables|Default|SetTotalItems (+ (Variables|Default|GetTotalItems) 1))
  (if (>= (Variables|Default|GetTotalItems) 5)
    (bind _asbp_my_char (Utilities|Casting|CastToBP_MyChar (Game|Player|GetPlayerPawn 0)))
    (Variables|/Game/MyContent/Blueprints/BP_MyChar.BP_MyChar_C|SetFullBag _asbp_my_char true)))